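; BP_Spawners is a zombie spawner that periodically adds BP_AI actors to the scene.
; On BeginPlay it starts a looping five-second timer that calls Spawn.
; Spawn places an AI at the Sphere component's location, ignoring collisions, and increments ZombiesInScene until it reaches a fixed cap.
; Nothing in this Blueprint decrements that counter.
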(event EventBeginPlay
  (Utilities|Time|SetTimerbyFunctionName 0 "Spawn" 5.0 true))

(fn ConstructionScript)

(fn Spawn
  (if (< (Variables|Default|GetZombiesInScene) 11)
    (Game|SpawnActorfromClass "/Game/Game/AI/BP_AI.BP_AI_C" (Math|Conversions|ToTransform(Vector) (Transformation|GetWorldLocation (Variables|Default|GetSphere))) "AlwaysSpawn" "MultiplyWithRoot" 0 0)
    (Variables|Default|SetZombiesInScene (+ (Variables|Default|GetZombiesInScene) 1))))