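; Replicated door actor that swings open and also hosts a win trigger for the match.
; The Door event plays a timeline that scales the OpenDoor value into the yaw of the Arrow component.
; Overlapping the Win volume calls WinCondition, which asks BP_ThirdPersonGameMode to evaluate the players.
; The Box overlap events are empty, leaving the character's interact-widget show and hide logic disconnected.
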(event OnComponentBeginOverlap(Win)
  (params (OverlappedComponent :type Primitive%20Component%20Object%20Reference) (OtherActor :type Actor%20Object%20Reference) (OtherComp :type Primitive%20Component%20Object%20Reference) (OtherBodyIndex :type Integer) (bFromSweep :type Boolean) (SweepResult :type Hit%20Result%20Structure%20%28by%20ref%29))
  ;[0.15 0.15 0.15 0.5] 1
  (CallFunction|WinCondition))

(event OnComponentBeginOverlap(Box)
  (params (OverlappedComponent :type Primitive%20Component%20Object%20Reference) (OtherActor :type Actor%20Object%20Reference) (OtherComp :type Primitive%20Component%20Object%20Reference) (OtherBodyIndex :type Integer) (bFromSweep :type Boolean) (SweepResult :type Hit%20Result%20Structure%20%28by%20ref%29)))

(event OnComponentEndOverlap(Box)
  (params (OverlappedComponent :type Primitive%20Component%20Object%20Reference) (OtherActor :type Actor%20Object%20Reference) (OtherComp :type Primitive%20Component%20Object%20Reference) (OtherBodyIndex :type Integer)))

(event Custom|Door
  (bind _animdoor (Timeline|Timeline Play)
    (:Update
      (Transformation|SetRelativeRotation (Variables|Default|GetArrow) (Math|Rotator|MakeRotator 0.0 0.0 (* (Variables|Default|GetOpenDoor) _animdoor)) false false))))

(event Custom|WinCondition
  (params (PlayerWinner :type BP%20Third%20Person%20Character%20Object%20Reference))
  (bind _asbp_third_person_game_mode (Utilities|Casting|CastToBP_ThirdPersonGameMode (Game|GetGameMode)))
  (Default|EvaluatePlayers _asbp_third_person_game_mode))

(event EventBeginPlay
  (Networking|SetReplicates true))

(event Collision|EventActorBeginOverlap
  (params (OtherActor :type Actor%20Object%20Reference)))

(event EventTick
  (params (DeltaSeconds :type Float%20%28single-precision%29)))

(fn ConstructionScript)